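; EnemyController is an AI controller for the computer opponent in a turn-based game with a soccer ball.
; It runs the EnemyBT behavior tree on BeginPlay.
; When AI perception updates on a SoccerBall, it writes that ball to the BallObj blackboard key.
; GetTurn reports the enemy's turn as the inverse of IsTurn on the player's TopDownCharacter.
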(event OnTargetPerceptionUpdated(AIPerception)
  (params (Actor :type Actor%20Object%20Reference) (Stimulus :type AI%20Stimulus%20Structure))
  (bind _assoccer_ball (Utilities|Casting|CastToSoccerBall Actor))
  (AI|Components|Blackboard|SetValueasObject (AI|GetBlackboard 0) (Utilities|Name|MakeLiteralName "BallObj") _assoccer_ball))

(event EventBeginPlay
  (AI|RunBehaviorTree "/Game/Blueprints/EnemyBT.EnemyBT"))

(event EventTick
  (params (DeltaSeconds :type Float%20%28single-precision%29)))

(fn ConstructionScript)

(fn GetTurn
  (bind _astop_down_character (Utilities|Casting|CastToTopDownCharacter (Game|Player|GetPlayerPawn 0)))
  (return (not (Variables|/Game/Blueprints/TopDownCharacter.TopDownCharacter_C|GetisTurn _astop_down_character))))