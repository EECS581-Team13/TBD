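; Blueprint function library for the character editor that applies a saved facial appearance to a character mesh.
; ApplyMorphTargets reads the player-number row from the PlayerAppearance data table and collects its values into symmetric and single morph target arrays.
; Symmetric entries set both _Left and _Right morphs to the same value, while the others set one morph each, pairing names and values by array index.
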(fn ApplyMorphTargets
  (params (charParam :type Skeletal%20Mesh%20Actor%20Object%20Reference%20%28by%20ref%29) (playerNum :type String))
  (bind _lr_morphtargetvals (LocalVariables|GetLR_MorphTargetVals))
  (bind _skeletalmeshcomponent (Variables|/Script/Engine.SkeletalMeshActor|GetSkeletalMeshComponent charParam))
  (bind _morphtargetvals (LocalVariables|GetMorphTargetVals))
  ;[1 1 1] Apply morph target values from row <Player Num> in Player Appearance data table to <Char Param>
  (bind _returnvalue (Utilities|GetDataTableRow "/Game/DataAssets/Data_CSV/PlayerAppearance.PlayerAppearance" (Utilities|String|StringToName playerNum))
    (:then
      (Utilities|Array|Add _lr_morphtargetvals (.Blink (Utilities|Struct|BreakPlayerAppearance _returnvalue)))
      (Utilities|Array|Add _lr_morphtargetvals (.BrowsDown (Utilities|Struct|BreakPlayerAppearance _returnvalue)))
      (Utilities|Array|Add _lr_morphtargetvals (.BrownIn (Utilities|Struct|BreakPlayerAppearance _returnvalue)))
      (Utilities|Array|Add _lr_morphtargetvals (.BrowsOuterLower (Utilities|Struct|BreakPlayerAppearance _returnvalue)))
      (Utilities|Array|Add _lr_morphtargetvals (.BrowsUp (Utilities|Struct|BreakPlayerAppearance _returnvalue)))
      (Utilities|Array|Add _lr_morphtargetvals (.CheekPuff (Utilities|Struct|BreakPlayerAppearance _returnvalue)))
      (Utilities|Array|Add _lr_morphtargetvals (.EyesWide (Utilities|Struct|BreakPlayerAppearance _returnvalue)))
      (Utilities|Array|Add _lr_morphtargetvals (.Frown (Utilities|Struct|BreakPlayerAppearance _returnvalue)))
      (Utilities|Array|Add _lr_morphtargetvals (.JawRotateY (Utilities|Struct|BreakPlayerAppearance _returnvalue)))
      (Utilities|Array|Add _lr_morphtargetvals (.JawRotateZ (Utilities|Struct|BreakPlayerAppearance _returnvalue)))
      (Utilities|Array|Add _lr_morphtargetvals (.Jaw (Utilities|Struct|BreakPlayerAppearance _returnvalue)))
      (Utilities|Array|Add _lr_morphtargetvals (.LowerLipDown (Utilities|Struct|BreakPlayerAppearance _returnvalue)))
      (Utilities|Array|Add _lr_morphtargetvals (.Midmouth (Utilities|Struct|BreakPlayerAppearance _returnvalue)))
      (Utilities|Array|Add _lr_morphtargetvals (.MouthNarrow (Utilities|Struct|BreakPlayerAppearance _returnvalue)))
      (Utilities|Array|Add _lr_morphtargetvals (.MouthWhistle_NarrowAdjust (Utilities|Struct|BreakPlayerAppearance _returnvalue)))
      (Utilities|Array|Add _lr_morphtargetvals (.NoseScrunch (Utilities|Struct|BreakPlayerAppearance _returnvalue)))
      (Utilities|Array|Add _lr_morphtargetvals (.Smile (Utilities|Struct|BreakPlayerAppearance _returnvalue)))
      (Utilities|Array|Add _lr_morphtargetvals (.Squint (Utilities|Struct|BreakPlayerAppearance _returnvalue)))
      (Utilities|Array|Add _lr_morphtargetvals (.UpperLipUp (Utilities|Struct|BreakPlayerAppearance _returnvalue)))
      (Utilities|Array|Add _morphtargetvals (.JawBackward (Utilities|Struct|BreakPlayerAppearance _returnvalue)))
      (Utilities|Array|Add _morphtargetvals (.JawForeward (Utilities|Struct|BreakPlayerAppearance _returnvalue)))
      (Utilities|Array|Add _morphtargetvals (.Jaw_Down (Utilities|Struct|BreakPlayerAppearance _returnvalue)))
      (Utilities|Array|Add _morphtargetvals (.Jaw_Up (Utilities|Struct|BreakPlayerAppearance _returnvalue)))
      (Utilities|Array|Add _morphtargetvals (.LowerLipIn (Utilities|Struct|BreakPlayerAppearance _returnvalue)))
      (Utilities|Array|Add _morphtargetvals (.LowerLipOut (Utilities|Struct|BreakPlayerAppearance _returnvalue)))
      (Utilities|Array|Add _morphtargetvals (.MouthDown (Utilities|Struct|BreakPlayerAppearance _returnvalue)))
      (Utilities|Array|Add _morphtargetvals (.MouthOpen (Utilities|Struct|BreakPlayerAppearance _returnvalue)))
      (Utilities|Array|Add _morphtargetvals (.MouthUp (Utilities|Struct|BreakPlayerAppearance _returnvalue)))
      (Utilities|Array|Add _morphtargetvals (.TongueUp (Utilities|Struct|BreakPlayerAppearance _returnvalue)))
      (Utilities|Array|Add _morphtargetvals (.UpperLipIn (Utilities|Struct|BreakPlayerAppearance _returnvalue)))
      (Utilities|Array|Add _morphtargetvals (.UpperLipOut (Utilities|Struct|BreakPlayerAppearance _returnvalue)))
      (for (_array_element _array_index) (LocalVariables|GetLR_MorphTargets)
        (Components|SkeletalMesh|SetMorphTarget _skeletalmeshcomponent (Utilities|String|StringToName (Utilities|String|ToString(Text) (Utilities|Text|FormatText "{MorphName}_Right" (Utilities|Text|ToText(Name) _array_element)))) (Utilities|Array|Get(acopy) (LocalVariables|GetLR_MorphTargetVals) _array_index) true)
        (Components|SkeletalMesh|SetMorphTarget _skeletalmeshcomponent (Utilities|String|StringToName (Utilities|String|ToString(Text) (Utilities|Text|FormatText "{MorphName}_Left" (Utilities|Text|ToText(Name) _array_element)))) (Utilities|Array|Get(acopy) (LocalVariables|GetLR_MorphTargetVals) _array_index) true))
      (for (_array_element_2 _array_index_2) (LocalVariables|GetMorphTargets)
        (Components|SkeletalMesh|SetMorphTarget _skeletalmeshcomponent (Utilities|String|StringToName (Utilities|String|ToString(Text) (Utilities|Text|FormatText (Utilities|Text|ToText(Name) _array_element_2)))) (Utilities|Array|Get(acopy) (LocalVariables|GetMorphTargetVals) _array_index_2) true)))))